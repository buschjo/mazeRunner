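; Blue door Blueprint that opens once for a player character holding the blue key.
; Trigger overlap casts to ThirdPersonCharacter and checks GotBlueKey, playing a closed-door sound at the door if the key is missing.
; With the key, an IsAlreadyOpen flag blocks repeat openings, then the open sound plays and a timeline rotates the door.
; Each update lerps from the door's current relative rotation toward the open angle, rather than from a stored start.
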(event OnComponentBeginOverlap(Trigger)
  (params (OverlappedComponent :type Primitive%20Component%20Object%20Reference) (OtherActor :type Actor%20Object%20Reference) (OtherComp :type Primitive%20Component%20Object%20Reference) (OtherBodyIndex :type Integer) (bFromSweep :type Boolean) (SweepResult :type Hit%20Result%20Structure%20%28by%20ref%29))
  (bind _door (Variables|Default|GetDoor))
  ;[1 1 1] Check if door can be opened or not and play respective sound cues
  (bind _asthird_person_character (Utilities|Casting|CastToThirdPersonCharacter OtherActor))
  (if (Variables|/Game/ThirdPersonBP/Blueprints/ThirdPersonCharacter.ThirdPersonCharacter_C|GetGotBlueKey _asthird_person_character)
    (if (not (Variables|Default|GetisAlreadyOpen))
      (Variables|Default|SetisAlreadyOpen true)
      (CallFunction|MakeOpenDoorSound)
      (bind _open_the_door (Timeline|Timeline_0 PlayFromStart)
        (:Update
          (Transformation|SetRelativeRotation _door (Math|Rotator|Lerp(Rotator) (Variables|/Script/Engine.SceneComponent|GetRelativeRotation _door) "0,90.000000, 0" _open_the_door true) false false))))
    (else
      (CallFunction|MakeClosedDoorSound))))

(fn ConstructionScript)

(fn MakeClosedDoorSound
  (Audio|PlaySoundatLocation "/Game/Key_Door_Mechanics/closed_Cue.closed_Cue" (Transformation|GetWorldLocation (Variables|Default|GetDoor)) "0, 0, 0" 1.0 1.0 0.0 0 0 0))

(fn MakeOpenDoorSound
  (Audio|PlaySoundatLocation "/Game/Key_Door_Mechanics/open_Cue.open_Cue" (Transformation|GetWorldLocation (Variables|Default|GetDoor)) "0, 0, 0" 1.0 1.0 0.0 0 0 0))